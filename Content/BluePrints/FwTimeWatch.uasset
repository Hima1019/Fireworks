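; FwTimeWatch is a watch prop that displays elapsed time and the current round.
; SetTime turns the Time component's relative yaw in proportion to time over MaxTime, one full revolution at the maximum, keeping roll and pitch.
; SetRound resets the time to zero and swaps the mesh material to match round one, two or three.
; It has no Tick or BeginPlay logic, so it changes only when these functions are called.
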(event EventBeginPlay)

(event EventActorBeginOverlap
  (params (OtherActor :type Actor%20Object%20Reference)))

(event EventTick
  (params (DeltaSeconds :type Float%20%28single-precision%29)))

(fn ConstructionScript)

(fn SetTime
  (params (Time :type Float%20%28single-precision%29))
  (bind _relativerotation (Variables|/Script/Engine.SceneComponent|GetRelativeRotation (Variables|Default|GetTime)))
  (bind (_roll _pitch) (Math|Rotator|BreakRotator _relativerotation))
  (Transformation|SetRelativeRotation (Variables|Default|GetTime) (Math|Rotator|MakeRotator _roll _pitch (* (/ Time (Variables|Default|GetMaxTime)) 3.6e+02)) false false))

(fn SetRound
  (params (Round :type Integer))
  (bind _staticmeshcomponent (Variables|Debug|GetStaticMeshComponent))
  (CallFunction|SetTime 0.0)
  (switch int Round
    (:1
      (Rendering|Material|SetMaterial _staticmeshcomponent 0 "/Game/Architecture/Materials/M_Watch1.M_Watch1"))
    (:2
      (Rendering|Material|SetMaterial _staticmeshcomponent 0 "/Game/Architecture/Materials/M_Watch2.M_Watch2"))
    (:3
      (Rendering|Material|SetMaterial _staticmeshcomponent 0 "/Game/Architecture/Materials/M_Watch3.M_Watch3"))))