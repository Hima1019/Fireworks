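; FwBGM is a Blueprint that switches the game's background music components between title, rounds and results.
; RoundStart activates the component for the given round (one to three) and destroys the previous round's component.
; TitleEnd destroys the title component, and GameEnd destroys the Round 3 component and activates the Result one.
; Tracks are removed by destroying their components, and the event graph holds no logic.
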(event EventBeginPlay)

(event EventActorBeginOverlap
  (params (OtherActor :type Actor%20Object%20Reference)))

(event EventTick
  (params (DeltaSeconds :type Float%20%28single-precision%29)))

(fn ConstructionScript)

(fn RoundStart
  (params (Round :type Integer))
  (bind _round1 (Variables|Default|GetRound1))
  (bind _round2 (Variables|Default|GetRound2))
  (switch int Round
    (:1
      (Components|Activation|SetActive _round1 true false))
    (:2
      (Components|Activation|SetActive _round2 true false)
      (Components|DestroyComponent _round1))
    (:3
      (Components|Activation|SetActive (Variables|Default|GetRound3) true false)
      (Components|DestroyComponent _round2))))

(fn GameEnd
  (Components|DestroyComponent (Variables|Default|GetRound3))
  (Components|Activation|SetActive (Variables|Default|GetResult) true false))

(fn TitleEnd
  (Components|DestroyComponent (Variables|Default|GetTitle)))