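; FwBoardBall is a board-side ball that absorbs an overlapping, visible FwPlaneBall.
; On overlap it copies the plane ball's SeedColor through ChangeColor, which applies a dynamic material instance, then destroys that ball.
; A hidden board ball then becomes visible, while an already visible one calls EnterBoard on the first FwPlayerController found.
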(event OnComponentBeginOverlap(StaticMeshComponent)
  (params (OtherActor :type Actor%20Object%20Reference) (OtherComp :type Primitive%20Component%20Object%20Reference) (OtherBodyIndex :type Integer) (bFromSweep :type Boolean) (SweepResult :type Hit%20Result%20Structure%20%28by%20ref%29))
  (bind _staticmeshcomponent (Variables|Debug|GetStaticMeshComponent))
  (bind _asfw_plane_ball (Utilities|Casting|CastToFwPlaneBall OtherActor))
  (if (Rendering|IsVisible (Variables|/Script/Engine.StaticMeshActor|GetStaticMeshComponent _asfw_plane_ball))
    (CallFunction|ChangeColor (Variables|/Game/BluePrints/FwPlaneBall.FwPlaneBall_C|GetSeedColor _asfw_plane_ball))
    (Actor|DestroyActor _asfw_plane_ball)
    (if (Rendering|IsVisible _staticmeshcomponent)
      (bind _outactors (Actor|GetAllActorsOfClass "/Game/BluePrints/FwPlayerController.FwPlayerController_C"))
      (Default|EnterBoard (Utilities|Array|Get(acopy) _outactors))
      (else
        (Rendering|SetVisibility _staticmeshcomponent true false)))))

(event EventTick
  (params (DeltaSeconds :type Float%20%28single-precision%29)))

(event EventBeginPlay)

(fn ConstructionScript)

(fn ChangeColor
  (params (Color :type Linear%20Color%20Structure))
  (Variables|Default|SetSeedColor Color)
  ;[1 1 1] 色変更
  (bind _returnvalue (Rendering|Material|CreateDynamicMaterialInstance (Variables|Debug|GetStaticMeshComponent) 0 "/Game/Architecture/Materials/Mo_Ball_Inst.Mo_Ball_Inst" :!class /Script/Engine.PrimitiveComponent))
  (Rendering|Material|SetVectorParameterValue _returnvalue "BaseColor" Color :!class /Script/Engine.MaterialInstanceDynamic))