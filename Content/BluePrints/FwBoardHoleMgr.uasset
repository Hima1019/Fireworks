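; FwBoardHoleMgr is a scene component that manages the firework balls in a board's holes.
; On BeginPlay it picks a random enable pattern, toggles child visibility, and gives visible balls a random color, a round-dependent shell type and a matching gunpowder texture.
; EnterBoard destroys hidden board balls.
; PlaneHitCheck and AllDestroyBall walk sibling managers to hit-test visible balls against the base board's rotation or destroy them.
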(event Custom|SelectPattern
  ;[1 1 1] 板パターン登録
  (bind _output_get (Variables|ボール設定|SetPatternNo (Math|Random|RandomInteger (Variables|ボール設定|GetMaxPattern))))
  (switch int _output_get
    (:Default
      (Variables|ボール設定|SetEnableList (Variables|ボール設定|GetEnablePattern0)))
    (:0
      (Variables|ボール設定|SetEnableList (Variables|ボール設定|GetEnablePattern0)))
    (:1
      (Variables|ボール設定|SetEnableList (Variables|ボール設定|GetEnablePattern1)))
    (:2
      (Variables|ボール設定|SetEnableList (Variables|ボール設定|GetEnablePattern2)))
    (:3
      (Variables|ボール設定|SetEnableList (Variables|ボール設定|GetEnablePattern3)))
    (:4
      (Variables|ボール設定|SetEnableList (Variables|ボール設定|GetEnablePattern4)))
    (:5
      (Variables|ボール設定|SetEnableList (Variables|ボール設定|GetEnablePattern5)))
    (:6
      (Variables|ボール設定|SetEnableList (Variables|ボール設定|GetEnablePattern6)))
    (:7
      (Variables|ボール設定|SetEnableList (Variables|ボール設定|GetEnablePattern7)))))

(event Custom|EnterBoard
  ;[1 1 1] 非表示状態のものは削除
  (Variables|Default|SetType "NewEnumerator1")
  (for _array_element (Components|GetChildrenComponents (VehicleSound|GetRootComponent (Components|GetOwner)) false)
    (bind _asfw_board_hole_mgr (Utilities|Casting|CastToFwBoardHoleMgr _array_element))
    (for _array_element_2 (Components|GetChildrenComponents _asfw_board_hole_mgr false)
      (bind _asfw_board_ball (Utilities|Casting|CastToFwBoardBall (Variables|/Script/Engine.ChildActorComponent|GetChildActor (.AsChild%20Actor%20Component (Utilities|Casting|CastToChildActorComponent _array_element_2)))))
      (if (Variables|/Script/Engine.SceneComponent|GetbVisible (Variables|/Script/Engine.StaticMeshActor|GetStaticMeshComponent _asfw_board_ball))
        (if (Utilities|Enum|Equal(Enum) (Variables|Default|GetType) "NewEnumerator0")
          (Variables|Default|SetType (Variables|/Game/BluePrints/FwBoardBall.FwBoardBall_C|GetType _asfw_board_ball)))
        (else
          (Actor|DestroyActor _asfw_board_ball))))))

(event EventBeginPlay
  (bind _colorlist (Variables|ボール設定|GetColorList))
  (CallFunction|SelectPattern)
  (Variables|Default|SetHuleMun (Utilities|Array|Length (Components|GetChildrenComponents false)))
  ;[1 1 1] 描画切り替え
  (for (_array_element _array_index) (Variables|ボール設定|GetEnableList)
    (if (< _array_index (Variables|Default|GetHuleMun))
      (Rendering|SetVisibility (Utilities|Array|Get(acopy) (Components|GetChildrenComponents false) _array_index) _array_element true)
      (if _array_element
        (bind _asfw_plane_ball (Utilities|Casting|CastToFwPlaneBall (Variables|/Script/Engine.ChildActorComponent|GetChildActor (.AsChild%20Actor%20Component (Utilities|Casting|CastToChildActorComponent (Utilities|Array|Get(acopy) (Components|GetChildrenComponents false) _array_index))))))
        (Default|ChangeColor _asfw_plane_ball (Utilities|Array|Get(acopy) _colorlist (Math|Random|RandomInteger (Utilities|Array|Length _colorlist))))
        (switch int (Variables|/Game/BluePrints/FwPlayerController.FwPlayerController_C|GetRound (.AsFw%20Player%20Controller (Utilities|Casting|CastToFwPlayerController (Game|GetPlayerController 0))))
          (:1
            (switch int (Math|Random|RandomInteger 3)
              (:Default
                (Variables|/Game/BluePrints/FwPlaneBall.FwPlaneBall_C|SetType _asfw_plane_ball "NewEnumerator0" :!label _label))
              (:0
                (goto _label))
              (:1
                (Variables|/Game/BluePrints/FwPlaneBall.FwPlaneBall_C|SetType _asfw_plane_ball "NewEnumerator2"))
              (:2
                (Variables|/Game/BluePrints/FwPlaneBall.FwPlaneBall_C|SetType _asfw_plane_ball "NewEnumerator3"))))
          (:2
            (switch int (Math|Random|RandomInteger 2)
              (:Default
                (goto _label))
              (:0
                (Variables|/Game/BluePrints/FwPlaneBall.FwPlaneBall_C|SetType _asfw_plane_ball "NewEnumerator0"))
              (:1
                (Variables|/Game/BluePrints/FwPlaneBall.FwPlaneBall_C|SetType _asfw_plane_ball "NewEnumerator5"))))
          (:3
            (switch int (Math|Random|RandomInteger 3)
              (:Default
                (goto _label))
              (:0
                (Variables|/Game/BluePrints/FwPlaneBall.FwPlaneBall_C|SetType _asfw_plane_ball "NewEnumerator0"))
              (:1
                (Variables|/Game/BluePrints/FwPlaneBall.FwPlaneBall_C|SetType _asfw_plane_ball "NewEnumerator1"))
              (:2
                (Variables|/Game/BluePrints/FwPlaneBall.FwPlaneBall_C|SetType _asfw_plane_ball "NewEnumerator4")))))
        (switch Utilities|FlowControl|Switch|SwitchonFwoFWActionEnum (Variables|/Game/BluePrints/FwPlaneBall.FwPlaneBall_C|GetType _asfw_plane_ball)
          (:NewEnumerator0
            (Rendering|Material|SetTextureParameterValue (Variables|/Game/BluePrints/FwPlaneBall.FwPlaneBall_C|GetDynamincMaterial _asfw_plane_ball) "Texture" "/Game/Architecture/Textures/kayaku01.kayaku01"))
          (:NewEnumerator1
            (Rendering|Material|SetTextureParameterValue (Variables|/Game/BluePrints/FwPlaneBall.FwPlaneBall_C|GetDynamincMaterial _asfw_plane_ball) "Texture" "/Game/Architecture/Textures/kayaku02.kayaku02"))
          (:NewEnumerator2
            (Rendering|Material|SetTextureParameterValue (Variables|/Game/BluePrints/FwPlaneBall.FwPlaneBall_C|GetDynamincMaterial _asfw_plane_ball) "Texture" "/Game/Architecture/Textures/kayaku03.kayaku03"))
          (:NewEnumerator3
            (Rendering|Material|SetTextureParameterValue (Variables|/Game/BluePrints/FwPlaneBall.FwPlaneBall_C|GetDynamincMaterial _asfw_plane_ball) "Texture" "/Game/Architecture/Textures/kayaku04.kayaku04"))
          (:NewEnumerator4
            (Rendering|Material|SetTextureParameterValue (Variables|/Game/BluePrints/FwPlaneBall.FwPlaneBall_C|GetDynamincMaterial _asfw_plane_ball) "Texture" "/Game/Architecture/Textures/kayaku05.kayaku05"))
          (:NewEnumerator5
            (Rendering|Material|SetTextureParameterValue (Variables|/Game/BluePrints/FwPlaneBall.FwPlaneBall_C|GetDynamincMaterial _asfw_plane_ball) "Texture" "/Game/Architecture/Textures/kayaku06.kayaku06")))))))

(event EventTick
  (params (DeltaSeconds :type Float%20%28single-precision%29)))

(fn PlaneHitCheck
  (bind _outactors (Actor|GetAllActorsOfClass "/Game/BluePrints/FwBaseBoard.FwBaseBoard_C"))
  (LocalVariables|SetRotation (Transformation|GetActorRotation (Utilities|Array|Get(acopy) _outactors)))
  (for _array_element (Components|GetChildrenComponents (VehicleSound|GetRootComponent (Components|GetOwner)) false)
    (bind _asfw_board_hole_mgr (Utilities|Casting|CastToFwBoardHoleMgr _array_element))
    (for _array_element_2 (Components|GetChildrenComponents _asfw_board_hole_mgr false)
      (bind _asfw_plane_ball (Utilities|Casting|CastToFwPlaneBall (Variables|/Script/Engine.ChildActorComponent|GetChildActor (.AsChild%20Actor%20Component (Utilities|Casting|CastToChildActorComponent _array_element_2)))))
      (if (Variables|/Script/Engine.SceneComponent|GetbVisible (Variables|/Script/Engine.StaticMeshActor|GetStaticMeshComponent _asfw_plane_ball))
        (bind _ishit (Default|HitCheck _asfw_plane_ball (LocalVariables|GetRotation)))
        (if _ishit
          (LocalVariables|SetIsCheck true)))))
  (return (LocalVariables|GetIsCheck)))

(fn AllDestroyBall
  ;[1 1 1] 表示されている玉削除
  (for _array_element (Components|GetChildrenComponents (VehicleSound|GetRootComponent (Components|GetOwner)) false)
    (bind _asfw_board_hole_mgr (Utilities|Casting|CastToFwBoardHoleMgr _array_element))
    (for _array_element_2 (Components|GetChildrenComponents _asfw_board_hole_mgr false)
      (bind _asfw_plane_ball (Utilities|Casting|CastToFwPlaneBall (Variables|/Script/Engine.ChildActorComponent|GetChildActor (.AsChild%20Actor%20Component (Utilities|Casting|CastToChildActorComponent _array_element_2)))))
      (if (Variables|/Script/Engine.SceneComponent|GetbVisible (Variables|/Script/Engine.StaticMeshActor|GetStaticMeshComponent _asfw_plane_ball))
        (Actor|DestroyActor _asfw_plane_ball)))))