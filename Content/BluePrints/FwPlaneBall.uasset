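; FwPlaneBall is a colored ball actor that can detect whether a visible FwBoardBall lies beneath it relative to a board's orientation.
; ChangeColor stores the seed color and applies it through a dynamic material instance of M_TexBall_Inst.
; HitCheck runs a short Visibility line trace along the rotated board's down vector, returning true only when it hits an FwBoardBall with a visible mesh.
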(event EventTick
  (params (DeltaSeconds :type Float%20%28single-precision%29)))

(event EventBeginPlay)

(fn ConstructionScript)

(fn ChangeColor
  (params (Color :type Linear%20Color%20Structure))
  (Variables|Default|SetSeedColor Color)
  ;[1 1 1] 色変更
  (bind _returnvalue (Rendering|Material|CreateDynamicMaterialInstance (Variables|Debug|GetStaticMeshComponent) 0 "/Game/Architecture/Materials/M_TexBall_Inst.M_TexBall_Inst" :!class /Script/Engine.PrimitiveComponent))
  (Rendering|Material|SetVectorParameterValue _returnvalue "BaseColor" Color :!class /Script/Engine.MaterialInstanceDynamic))

(fn HitCheck
  (params (BoardRotation :type Rotator))
  (bind _returnvalue (Transformation|GetActorLocation))
  (bind _outhit (Collision|LineTraceByChannel _returnvalue (+ _returnvalue (* (Math|Vector|GetUpVector BoardRotation) -15.0)) "TraceTypeQuery1" false 0 "None"))
  (bind _asfw_board_ball (Utilities|Casting|CastToFwBoardBall (.HitActor (Collision|BreakHitResult _outhit)))
    (:then
      (if (Variables|/Script/Engine.SceneComponent|GetbVisible (Variables|/Script/Engine.StaticMeshActor|GetStaticMeshComponent _asfw_board_ball))
        (return true)
        (else
          _)))
    (:CastFailed
      _))
  (return false))