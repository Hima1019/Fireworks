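; Player controller for a board game where a plane holding balls is rotated in 60-degree steps and lowered onto a board.
; BeginPlay caches the custom camera manager, finds the first FwBaseBoard and spawns an FwPlane offset above it.
; Left/right input starts a rotation that Tick animates, clamped to the remaining angle; Enter lowers the plane by the offset, and both are ignored mid-rotation.
; Debug mouse look feeds yaw and pitch to the camera manager.
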(event EventBeginPlay
  (Utilities|FlowControl|Sequence
    (:then_0
      ;[1 1 1] CameraManagerの登録
      (bind _asfw_player_camera_manager (Utilities|Casting|CastToFwPlayerCameraManager (Variables|Default|GetPlayerCameraManager)))
      (Variables|Default|SetMyCameraManager _asfw_player_camera_manager))
    (:then_1
      ;[1 1 1] レベルに設置されたFwBoard（作業台）を取得
      (bind _outactors (Actor|GetAllActorsOfClass "/Game/BluePrints/FwBaseBoard.FwBaseBoard_C"))
      (Variables|Default|SetBoardActor (Utilities|Array|Get(acopy) _outactors)))
    (:then_2
      ;[1 1 1] FwPlane（玉がはまってるやつ）を生成
      (bind _returnvalue (Game|SpawnActorfromClass "/Game/BluePrints/FwPlane.FwPlane_C" (Transformation|GetActorTransform (Variables|Default|GetBoardActor)) "Undefined" 0 0))
      (bind _output_get (Variables|Default|SetPlaneActor _returnvalue))
      (Transformation|AddActorLocalOffset _output_get (Math|Vector|MakeVector 0.0 0.0 (Variables|Default|GetPlaneOffset)) false false))))

(event EventTick
  (params (DeltaSeconds :type Float%20%28single-precision%29))
  (bind _rotationspeed (Variables|Rotation|GetRotationSpeed))
  (bind _planeactor (Variables|Default|GetPlaneActor))
  (bind _returnvalue (* DeltaSeconds _rotationspeed))
  (Utilities|FlowControl|Sequence
    (:then_0
      ;[1 1 1] 回転反映
      (if (Variables|Rotation|GetIsRotationRight)
        (Transformation|AddActorLocalRotation _planeactor (Math|Rotator|MakeRotator 0.0 0.0 (Math|Float|Min(Float) _returnvalue (Variables|Rotation|GetRotationValue))) false false)
        (bind _output_get (Variables|Rotation|SetRotationValue (- (Variables|Rotation|GetRotationValue) (Math|Float|Min(Float) _returnvalue (Variables|Rotation|GetRotationValue)))))
        (if (<= _output_get 0.0)
          (Variables|Rotation|SetIsRotationRight false))))
    (:then_1
      (if (Variables|Rotation|GetIsRotationLeft)
        (Transformation|AddActorLocalRotation _planeactor (Math|Rotator|MakeRotator 0.0 0.0 (Math|Float|Max(Float) (* _returnvalue -1.0) (Variables|Rotation|GetRotationValue))) false false)
        (bind _output_get_2 (Variables|Rotation|SetRotationValue (- (Variables|Rotation|GetRotationValue) (Math|Float|Max(Float) (* _returnvalue -1.0) (Variables|Rotation|GetRotationValue)))))
        (if (>= _output_get_2 0.0)
          (Variables|Rotation|SetIsRotationLeft false))))))

(event Input|ActionEvents|InputActionRotationLeft
  (params (Key :type Key%20Structure :default "AnyKey"))
  ;[1 1 1] 回転開始
  (:Pressed
    (if (not (or (Variables|Rotation|GetIsRotationLeft) (Variables|Rotation|GetIsRotationRight)))
      (Variables|Rotation|SetRotationValue -6e+01)
      (Variables|Rotation|SetIsRotationLeft true))))

(event Input|ActionEvents|InputActionRotationRight
  (params (Key :type Key%20Structure :default "AnyKey"))
  ;[1 1 1] 回転開始
  (:Pressed
    (if (not (or (Variables|Rotation|GetIsRotationLeft) (Variables|Rotation|GetIsRotationRight)))
      (Variables|Rotation|SetRotationValue 6e+01)
      (Variables|Rotation|SetIsRotationRight true))))

(event Input|ActionEvents|InputActionEnter
  (params (Key :type Key%20Structure :default "AnyKey"))
  (:Pressed
    (if (not (or (Variables|Rotation|GetIsRotationLeft) (Variables|Rotation|GetIsRotationRight)))
      (Transformation|AddActorLocalOffset (Variables|Default|GetPlaneActor) (Math|Vector|MakeVector 0.0 0.0 (* -1 (Variables|Default|GetPlaneOffset))) false false))))

(event Input|AxisEvents|InputAxisLookRight
  (params (AxisValue :type Float%20%28single-precision%29))
  ;[1 1 1] デバッグ用のマウス視線シミュレート
  (Default|AddYawInput (Variables|Default|GetMyCameraManager) AxisValue))

(event Input|AxisEvents|InputAxisLookUp
  (params (AxisValue :type Float%20%28single-precision%29))
  ;[1 1 1] デバッグ用のマウス視線シミュレート
  (Default|AddPitchInput (Variables|Default|GetMyCameraManager) AxisValue))

(fn ConstructionScript)