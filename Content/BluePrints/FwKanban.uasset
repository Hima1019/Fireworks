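; FwKanban is a signboard actor in a fireworks game that carries the title display and the result display.
; TitleEnd destroys the Title and TitleLogo components.
; ResultSet shows the Result widget, reads FireSeedCount from the first FwoFireWorksGenerator found in the level, and passes one of six tiered Japanese verdict lines to its ResultHUD.
; Its event graph and construction script are empty, and nothing in the file calls either function.
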(event EventBeginPlay)

(event EventActorBeginOverlap
  (params (OtherActor :type Actor%20Object%20Reference)))

(event EventTick
  (params (DeltaSeconds :type Float%20%28single-precision%29)))

(fn ConstructionScript)

(fn TitleEnd
  (Components|DestroyComponent (Variables|Default|GetTitle))
  (Components|DestroyComponent (Variables|Default|GetTitleLogo)))

(fn ResultSet
  (bind _result (Variables|Default|GetResult))
  (bind _returnvalue (UserInterface|GetUserWidgetObject _result))
  (bind _asresult_hud (Utilities|Casting|CastToResultHUD _returnvalue))
  (Rendering|SetVisibility _result true false)
  (bind _outactors (Actor|GetAllActorsOfClass "/Game/BluePrints/OikawaBP/FwoFireWorksGenerator.FwoFireWorksGenerator_C"))
  (if (< (Variables|/Game/BluePrints/OikawaBP/FwoFireWorksGenerator.FwoFireWorksGenerator_C|GetFireSeedCount (Utilities|Array|Get(acopy) _outactors)) 50)
    (Default|SetResult _asresult_hud "「まだまだじゃな」")
    (elif (< (Variables|/Game/BluePrints/OikawaBP/FwoFireWorksGenerator.FwoFireWorksGenerator_C|GetFireSeedCount (Utilities|Array|Get(acopy) _outactors)) 70)
      (Default|SetResult _asresult_hud "「まあまあじゃな」")
      (elif (< (Variables|/Game/BluePrints/OikawaBP/FwoFireWorksGenerator.FwoFireWorksGenerator_C|GetFireSeedCount (Utilities|Array|Get(acopy) _outactors)) 100)
        (Default|SetResult _asresult_hud "「なかなかやるな！」")
        (elif (< (Variables|/Game/BluePrints/OikawaBP/FwoFireWorksGenerator.FwoFireWorksGenerator_C|GetFireSeedCount (Utilities|Array|Get(acopy) _outactors)) 150)
          (Default|SetResult _asresult_hud "「上出来じゃ！！」")
          (elif (< (Variables|/Game/BluePrints/OikawaBP/FwoFireWorksGenerator.FwoFireWorksGenerator_C|GetFireSeedCount (Utilities|Array|Get(acopy) _outactors)) 200)
            (Default|SetResult _asresult_hud "「素晴らしい！」")
            (else
              (Default|SetResult _asresult_hud "「弟子にして下さい」"))))))))