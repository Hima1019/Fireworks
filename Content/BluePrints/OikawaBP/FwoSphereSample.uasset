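; Sample firework sphere actor built from FwoPlane child actors, gathered into an array on BeginPlay and launched once by the Fire event.
; Fire first shows each plane, activates a BOTAN component on it and disables collision on its seeds and meshes.
; It then boosts emission and launches each plane's appearance and FwoFireSeed child actors as physics bodies, sharing one random upward impulse per plane.
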(event Custom|Fire
  (Utilities|FlowControl|DoOnce false
    (:Completed
      (for _array_element (Variables|Default|GetPlaneArray)
        (Rendering|SetVisibility (Variables|/Game/BluePrints/OikawaBP/FwoPlane.FwoPlane_C|GetAppearance _array_element) true false)
        (bind _returnvalue (AddComponent|AddFwoABOTAN _array_element true))
        (Components|Activation|SetActive _returnvalue true false)
        (for _array_element_2 (Components|GetChildrenComponents (Variables|/Game/BluePrints/OikawaBP/FwoPlane.FwoPlane_C|GetDefaultSceneRoot _array_element) false)
          (bind _aschild_actor_component (Utilities|Casting|CastToChildActorComponent _array_element_2)
            (:then
              (bind _asfwo_fire_seed (Utilities|Casting|CastToFwoFireSeed (Variables|/Script/Engine.ChildActorComponent|GetChildActor _aschild_actor_component)))
              (Collision|SetActorEnableCollision _asfwo_fire_seed false))
            (:CastFailed
              (bind _asスタティックメッシュコンポーネント (Utilities|Casting|CastToStaticMeshComponent _array_element_2))
              (Collision|SetCollisionEnabled _asスタティックメッシュコンポーネント "NoCollision")))))
      (for _array_element_3 (Variables|Default|GetPlaneArray)
        (Variables|/Game/BluePrints/OikawaBP/FwoPlane.FwoPlane_C|SetAppearanceEmit _array_element_3 1e+03)
        (Variables|Default|SetUpForce (Math|Vector|MakeVector 0.0 0.0 (Math|Random|RandomFloatinRange (Variables|Default|GetimpulseMin) (Variables|Default|GetimpulseMax))))
        (for _array_element_4 (Components|GetChildrenComponents (VehicleSound|GetRootComponent _array_element_3) false)
          ;[1 1 1] シード発射
          (bind _aschild_actor_component_2 (Utilities|Casting|CastToChildActorComponent _array_element_4))
          (bind _asfwo_fire_seed_2 (Utilities|Casting|CastToFwoFireSeed (Variables|/Script/Engine.ChildActorComponent|GetChildActor _aschild_actor_component_2)))
          (Physics|SetSimulatePhysics (Variables|/Script/Engine.StaticMeshActor|GetStaticMeshComponent _asfwo_fire_seed_2) true)
          (Physics|AddImpulse (Variables|/Script/Engine.StaticMeshActor|GetStaticMeshComponent _asfwo_fire_seed_2) (Variables|Default|GetUpForce) "None" false))
        ;[1 1 1] 外見発射
        (Physics|SetSimulatePhysics (Variables|/Game/BluePrints/OikawaBP/FwoPlane.FwoPlane_C|GetAppearance _array_element_3) true)
        (Physics|AddImpulse (Variables|/Game/BluePrints/OikawaBP/FwoPlane.FwoPlane_C|GetAppearance _array_element_3) (Variables|Default|GetUpForce) "None" false)))))

(event EventBeginPlay
  (for _array_element (Components|GetChildrenComponents (Variables|Default|GetDefaultSceneRoot) false)
    (Utilities|Array|Add (Variables|Default|GetPlaneArray) (.AsFwo%20Plane (Utilities|Casting|CastToFwoPlane (Variables|/Script/Engine.ChildActorComponent|GetChildActor (.AsChild%20Actor%20Component (Utilities|Casting|CastToChildActorComponent _array_element))))))))

(event EventActorBeginOverlap
  (params (OtherActor :type Actor%20Object%20Reference)))

(event EventTick
  (params (DeltaSeconds :type Float%20%28single-precision%29)))

(fn ConstructionScript)