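; FwoSrelializeFire keeps a bounded pool of saved stock entries and hands back a random one.
; AddStack grows SaveStocks up to ArrayMax, then overwrites at ArrayHead as a ring buffer, with a hard-coded wrap after index 19.
; GetStock filters SaveStocks into EnableArray, which it never clears, and picks a random index with the array length as the inclusive maximum, one past the end.
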(fn GetStock
  (bind _enablearray (LocalVariables|GetEnableArray))
  (if (== (Utilities|Array|Length (Variables|Default|GetSaveStocks)) 0)
    (return 0)
    (else
      (for _array_element (Variables|Default|GetSaveStocks)
        (if (not (== _array_element 0))
          (Utilities|Array|Add _enablearray _array_element)))
      (return (Utilities|Array|Get(acopy) _enablearray (Math|Random|RandomIntegerinRange 0 (Utilities|Array|Length _enablearray)))))))

(fn AddStack
  (params (NewParam :type Fwo%20Stock%20Object%20Reference))
  (bind _savestocks (Variables|Default|GetSaveStocks))
  (if (< (Utilities|Array|Length _savestocks) (Variables|Default|GetArrayMax))
    (Utilities|Array|Add _savestocks 0)
    (else
      (Utilities|Array|SetArrayElem _savestocks (Variables|Default|GetArrayHead) NewParam)
      (bind _result (Math|Integer|IncrementInt (Variables|Default|GetArrayHead))
        (:%20%20
          (if (> _result 19)
            (Variables|Default|SetArrayHead 0)))))))