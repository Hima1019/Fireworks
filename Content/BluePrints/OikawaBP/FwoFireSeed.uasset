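; Firework seed actor, apparently one star of a firework: a static mesh with an attached particle system that starts deactivated.
; FireStar works once, applying scale and mass scale, enabling physics and randomizing particle size, but never activating the particles.
; BeginPlay, Tick and FireStar share a change check on seed color and emissive strength that rebuilds the mesh's dynamic material.
; Helper functions expose particle visibility and linear damping.
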(event Custom|FireStar
  (params (particl :type Boolean))
  (bind _seedcolor (Variables|Default|GetSeedColor))
  (bind _emmit (Variables|Default|GetEmmit))
  (bind _alpha (Variables|Default|GetAlpha))
  (Utilities|FlowControl|DoOnce false
    (:Completed
      (Utilities|FlowControl|Sequence
        (:then_0
          (CallFunction|Scaling (Variables|Default|GetSeedScale))
          (CallFunction|MassScaling (Variables|Default|GetMassScale))
          (Physics|SetSimulatePhysics (Variables|Debug|GetStaticMeshComponent) true)
          (CallFunction|ParticlScaling (Math|Random|RandomFloatinRange 3.0 1e+01)))
        (:then_1
          (if (Math|Boolean|ORBoolean (Math|Vector|NotEqual(Vector) (Math|Conversions|ToVector(LinearColor) (Variables|Default|GetseedColorLog)) (Math|Conversions|ToVector(LinearColor) (Variables|Default|GetSeedColor)) 0.0001) (!= (Variables|Default|GetEmmitLog) (Variables|Default|GetEmmit)) false false)
            ;[1 1 1] 色変更
            (bind _returnvalue (Rendering|Material|CreateDynamicMaterialInstance (Variables|Debug|GetStaticMeshComponent) 0 "/Game/Architecture/Materials/Mo_Ball_Inst.Mo_Ball_Inst" :!class /Script/Engine.PrimitiveComponent))
            (Rendering|Material|SetVectorParameterValue _returnvalue "BaseColor" _seedcolor :!class /Script/Engine.MaterialInstanceDynamic)
            (Variables|Default|SetseedColorLog _seedcolor)
            (Rendering|Material|SetVectorParameterValue _returnvalue "EmmitColor" (Variables|Default|GetEmmitColor) :!class /Script/Engine.MaterialInstanceDynamic)
            (Variables|Default|SetEmmitColorLog (Variables|Default|GetEmmitColor))
            (Rendering|Material|SetScalarParameterValue _returnvalue "Emmit" _emmit :!class /Script/Engine.MaterialInstanceDynamic)
            (Variables|Default|SetEmmitLog _emmit)
            (Rendering|Material|SetScalarParameterValue _returnvalue "Alpha" _alpha :!class /Script/Engine.MaterialInstanceDynamic)
            (Variables|Default|SetAlphaLog _alpha)
            (Variables|Default|SetEmmitColor (Variables|Default|GetSeedColor))))
        (:then_2
          (Utilities|FlowControl|Delay 2.0))))))

(event EventTick
  (params (DeltaSeconds :type Float%20%28single-precision%29))
  (bind _seedcolor (Variables|Default|GetSeedColor))
  (bind _emmit (Variables|Default|GetEmmit))
  (bind _alpha (Variables|Default|GetAlpha))
  (if (Math|Boolean|ORBoolean (Math|Vector|NotEqual(Vector) (Math|Conversions|ToVector(LinearColor) (Variables|Default|GetseedColorLog)) (Math|Conversions|ToVector(LinearColor) (Variables|Default|GetSeedColor)) 0.0001) (!= (Variables|Default|GetEmmitLog) (Variables|Default|GetEmmit)) false false)
    ;[1 1 1] 色変更
    (bind _returnvalue (Rendering|Material|CreateDynamicMaterialInstance (Variables|Debug|GetStaticMeshComponent) 0 "/Game/Architecture/Materials/Mo_Ball_Inst.Mo_Ball_Inst" :!class /Script/Engine.PrimitiveComponent))
    (Rendering|Material|SetVectorParameterValue _returnvalue "BaseColor" _seedcolor :!class /Script/Engine.MaterialInstanceDynamic)
    (Variables|Default|SetseedColorLog _seedcolor)
    (Rendering|Material|SetVectorParameterValue _returnvalue "EmmitColor" (Variables|Default|GetEmmitColor) :!class /Script/Engine.MaterialInstanceDynamic)
    (Variables|Default|SetEmmitColorLog (Variables|Default|GetEmmitColor))
    (Rendering|Material|SetScalarParameterValue _returnvalue "Emmit" _emmit :!class /Script/Engine.MaterialInstanceDynamic)
    (Variables|Default|SetEmmitLog _emmit)
    (Rendering|Material|SetScalarParameterValue _returnvalue "Alpha" _alpha :!class /Script/Engine.MaterialInstanceDynamic)
    (Variables|Default|SetAlphaLog _alpha)
    (Variables|Default|SetEmmitColor (Variables|Default|GetSeedColor))))

(event EventBeginPlay
  (bind _seedcolor (Variables|Default|GetSeedColor))
  (bind _emmit (Variables|Default|GetEmmit))
  (bind _alpha (Variables|Default|GetAlpha))
  (Components|Activation|Deactivate (Variables|コンポーネント|GetParticleSystem))
  (if (Math|Boolean|ORBoolean (Math|Vector|NotEqual(Vector) (Math|Conversions|ToVector(LinearColor) (Variables|Default|GetseedColorLog)) (Math|Conversions|ToVector(LinearColor) (Variables|Default|GetSeedColor)) 0.0001) (!= (Variables|Default|GetEmmitLog) (Variables|Default|GetEmmit)) false false)
    ;[1 1 1] 色変更
    (bind _returnvalue (Rendering|Material|CreateDynamicMaterialInstance (Variables|Debug|GetStaticMeshComponent) 0 "/Game/Architecture/Materials/Mo_Ball_Inst.Mo_Ball_Inst" :!class /Script/Engine.PrimitiveComponent))
    (Rendering|Material|SetVectorParameterValue _returnvalue "BaseColor" _seedcolor :!class /Script/Engine.MaterialInstanceDynamic)
    (Variables|Default|SetseedColorLog _seedcolor)
    (Rendering|Material|SetVectorParameterValue _returnvalue "EmmitColor" (Variables|Default|GetEmmitColor) :!class /Script/Engine.MaterialInstanceDynamic)
    (Variables|Default|SetEmmitColorLog (Variables|Default|GetEmmitColor))
    (Rendering|Material|SetScalarParameterValue _returnvalue "Emmit" _emmit :!class /Script/Engine.MaterialInstanceDynamic)
    (Variables|Default|SetEmmitLog _emmit)
    (Rendering|Material|SetScalarParameterValue _returnvalue "Alpha" _alpha :!class /Script/Engine.MaterialInstanceDynamic)
    (Variables|Default|SetAlphaLog _alpha)
    (Variables|Default|SetEmmitColor (Variables|Default|GetSeedColor))))

(fn ConstructionScript)

(fn Scaling
  (params (inScale :type Float%20%28single-precision%29))
  (bind _output_get (Variables|Default|SetSeedScale inScale))
  (Transformation|SetRelativeScale3D (Variables|Debug|GetStaticMeshComponent) (* (Transformation|GetWorldScale (Variables|Debug|GetStaticMeshComponent)) _output_get)))

(fn MassScaling
  (params (inMass :type Float%20%28single-precision%29))
  (bind _output_get (Variables|Default|SetMassScale inMass))
  (Class|PrimitiveComponent|SetMassScale (Variables|Debug|GetStaticMeshComponent) "None" _output_get))

(fn ParticlScaling
  (params (scale :type Float%20%28single-precision%29))
  (bind _output_get (Variables|Default|SetparticlScale scale))
  (if (< _output_get 0.0)
    (Components|Activation|Deactivate (Variables|コンポーネント|GetParticleSystem))
    (else
      (Transformation|SetWorldScale3D (Variables|コンポーネント|GetParticleSystem) (* (Math|Vector|MakeVector 1.0 1.0 1.0) _output_get)))))

(fn SetParticlActiv
  (params (flag :type Boolean))
  (bind _particlesystem (Variables|コンポーネント|GetParticleSystem))
  (bind _particlesystem_2 (Variables|コンポーネント|GetParticleSystem))
  (if flag
    (Components|Activation|Activate _particlesystem_2 true)
    (Rendering|SetVisibility _particlesystem_2 true false)
    (else
      (Components|Activation|Deactivate _particlesystem)
      (Rendering|SetVisibility _particlesystem false false))))

(fn Dumping
  (params (NewParam :type Float%20%28single-precision%29))
  (bind _output_get (Variables|Default|SetDumpingScale NewParam))
  (Class|PrimitiveComponent|SetLinearDamping (Variables|Debug|GetStaticMeshComponent) _output_get))