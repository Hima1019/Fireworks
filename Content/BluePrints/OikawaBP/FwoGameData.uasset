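; FwoGameData is a data Blueprint that keeps a capped pool of saved stock entries and hands one back at random.
; AddStack appends to SaveStocks until ArrayMax, then overwrites at ArrayHead and increments that index, with no wraparound.
; GetStock copies entries that differ from a compared value into EnableArray, then returns a random element.
; The random range runs up to the array length inclusive, so it can land one past the last element.
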(fn GetStock
  (bind _enablearray (LocalVariables|GetEnableArray))
  (if (== (Utilities|Array|Length (Variables|Default|GetSaveStocks)) 0)
    _
    (else
      (for _array_element (Variables|Default|GetSaveStocks)
        (if (not (== _array_element 0))
          (Utilities|Array|Add _enablearray _array_element)))))
  (return (Utilities|Array|Get(acopy) _enablearray (Math|Random|RandomIntegerinRange 0 (Utilities|Array|Length _enablearray)))))

(fn AddStack
  (bind _savestocks (Variables|Default|GetSaveStocks))
  (if (< (Utilities|Array|Length _savestocks) (Variables|Default|GetArrayMax))
    (Utilities|Array|Add _savestocks 0)
    (else
      (Utilities|Array|SetArrayElem _savestocks (Variables|Default|GetArrayHead) 0)
      (bind _result (Math|Integer|IncrementInt (Variables|Default|GetArrayHead))
        (:%20%20
          (Variables|Default|SetArrayHead _result)))))
  (return))