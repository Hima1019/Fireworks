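; Fireworks launcher Blueprint that shoots a given firework upward when RequestFire is called.
; RequestFire sets the firework's appearance emit value, then builds a vertical impulse from a random value between ImpulseMin and ImpulseMax.
; It enables physics and applies that upward impulse to each FwoFireSeed child actor under the firework's root, then to its Appearance component.
; The event graph and construction script have no active logic.
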(event EventBeginPlay)

(event EventActorBeginOverlap
  (params (OtherActor :type Actor%20Object%20Reference)))

(event EventTick
  (params (DeltaSeconds :type Float%20%28single-precision%29)))

(fn ConstructionScript)

(fn RequestFire
  (params (dictFireWorks :type Fwo%20Plane%20Object%20Reference))
  (bind _appearance (Variables|/Game/BluePrints/OikawaBP/FwoPlane.FwoPlane_C|GetAppearance dictFireWorks))
  (Variables|/Game/BluePrints/OikawaBP/FwoPlane.FwoPlane_C|SetAppearanceEmit dictFireWorks 1e+03)
  (LocalVariables|SetUpForce (* (Math|Vector|MakeVector 0.0 0.0 (Math|Random|RandomFloatinRange (Variables|Default|GetimpulseMin) (Variables|Default|GetimpulseMax))) (* 1.0 2.0)))
  (for _array_element (Components|GetChildrenComponents (VehicleSound|GetRootComponent dictFireWorks) false)
    ;[1 1 1] シード発射
    (bind _aschild_actor_component (Utilities|Casting|CastToChildActorComponent _array_element))
    (bind _asfwo_fire_seed (Utilities|Casting|CastToFwoFireSeed (Variables|/Script/Engine.ChildActorComponent|GetChildActor _aschild_actor_component)))
    (Physics|SetSimulatePhysics (Variables|/Script/Engine.StaticMeshActor|GetStaticMeshComponent _asfwo_fire_seed) true)
    (Physics|AddImpulse (Variables|/Script/Engine.StaticMeshActor|GetStaticMeshComponent _asfwo_fire_seed) (LocalVariables|GetUpForce) "None" false))
  ;[1 1 1] 外見発射
  (Physics|SetSimulatePhysics _appearance true)
  (Physics|AddImpulse _appearance (LocalVariables|GetUpForce) "None" false))