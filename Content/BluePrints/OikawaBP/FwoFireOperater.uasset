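; Firework firing operator that queues FwoStock actors and releases them to FwoFWLauncher actors at random intervals.
; PushStock spawns stocks scattered around the FwoFireStockPos point, and a Box2 overlap registers them in a pending list that reuses empty slots.
; On a randomized Tick countdown, it takes the first pending stock, moves it to its assigned launcher, requests fire with its Plene data, then destroys the stock.
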(event OnComponentBeginOverlap(Box2)
  (params (OtherActor :type Actor%20Object%20Reference) (OtherComp :type Primitive%20Component%20Object%20Reference) (OtherBodyIndex :type Integer) (bFromSweep :type Boolean) (SweepResult :type Hit%20Result%20Structure%20%28by%20ref%29))
  (CallFunction|PlaneRegister (.AsFwo%20Stock (Utilities|Casting|CastToFwoStock OtherActor))))

(event EventBeginPlay
  (bind _firedistance (Variables|Default|GetFireDistance))
  (bind (_x _y) (Math|Vector2D|BreakVector2D _firedistance))
  (bind _outactors (Actor|GetAllActorsOfClass "/Game/BluePrints/OikawaBP/FwoFWLauncher.FwoFWLauncher_C"))
  (Variables|Default|SetLauncherArray _outactors)
  (Variables|Default|SetspanTime (Math|Random|RandomFloatinRange _x _y))
  (bind _outactors_2 (Actor|GetAllActorsOfClass "/Game/BluePrints/OikawaBP/FwoFireStockPos.FwoFireStockPos_C"))
  (Variables|Default|SetStockPopPos (Transformation|GetActorTransform (Utilities|Array|Get(acopy) _outactors_2))))

(event EventTick
  (params (DeltaSeconds :type Float%20%28single-precision%29))
  (bind _firedistance (Variables|Default|GetFireDistance))
  (bind (_x _y) (Math|Vector2D|BreakVector2D _firedistance))
  (if (< (Variables|Default|GetspanTime) 0.0)
    (CallFunction|RunOperation)
    (Variables|Default|SetspanTime (Math|Random|RandomFloatinRange _x _y))
    (else
      (Variables|Default|SetspanTime (- (Variables|Default|GetspanTime) DeltaSeconds)))))

(fn ConstructionScript)

(fn PlaneRegister
  (params (NewParam :type Fwo%20Stock%20Object%20Reference))
  (bind _enableindex (CallFunction|GetEnableArraryItem true))
  (Utilities|Array|SetArrayElem (Variables|Default|GetPendingPlaneList) _enableindex NewParam))

(fn RunOperation
  (bind _enableindex (CallFunction|GetEnableArraryItem false))
  (if (== _enableindex -1)
    (return)
    (else
      (bind _output_get (Variables|Default|SetinsStock (Utilities|Array|Get(acopy) (Variables|Default|GetPendingPlaneList) _enableindex)))
      ;[1 1 1] 発射地点移動
      (Transformation|SetActorRelativeLocation _output_get (Transformation|GetActorLocation (Utilities|Array|Get(acopy) (Variables|Default|GetLauncherArray) (Variables|/Game/BluePrints/OikawaBP/FwoPlane.FwoPlane_C|GetLauncherId (Variables|/Game/BluePrints/OikawaBP/FwoStock.FwoStock_C|Getplene (Variables|Default|GetinsStock))))) false true)
      ;[1 1 1] 発射
      (Default|RequestFire (Utilities|Array|Get(acopy) (Variables|Default|GetLauncherArray) (Variables|/Game/BluePrints/OikawaBP/FwoPlane.FwoPlane_C|GetLauncherId (Variables|/Game/BluePrints/OikawaBP/FwoStock.FwoStock_C|Getplene (Variables|Default|GetinsStock)))) (Variables|/Game/BluePrints/OikawaBP/FwoStock.FwoStock_C|Getplene (Variables|Default|GetinsStock)))
      (Utilities|Array|RemoveItem (Variables|Default|GetPendingPlaneList) (Variables|Default|GetinsStock))
      (Actor|DestroyActor (Variables|Default|GetinsStock)))))

(fn PushStock
  (params (NewParam :type Fwo%20Plane%20Object%20Reference) (NewParam1 :type Linear%20Color%20Structure))
  (bind _stockpoppos (Variables|Default|GetStockPopPos))
  (bind (_location _rotation _scale) (Math|Transform|BreakTransform _stockpoppos))
  (bind _returnvalue (Game|SpawnActorfromClass "/Game/BluePrints/OikawaBP/FwoStock.FwoStock_C" (Math|Transform|MakeTransform (+ (* (Math|Random|RandomUnitVector) (Variables|Default|GetposRandomArea)) _location) _rotation _scale) "Undefined" 0 0))
  (Default|Make _returnvalue (Variables|/Game/BluePrints/OikawaBP/FwoPlane.FwoPlane_C|GetFireType NewParam) NewParam1)
  (Variables|/Game/BluePrints/OikawaBP/FwoStock.FwoStock_C|Setplene _returnvalue NewParam))

(fn GetEnableArraryItem
  (params (GetEnable :type Boolean))
  (bind _pendingplanelist (Variables|Default|GetPendingPlaneList))
  (if GetEnable
    (for (_array_element _array_index) (Variables|Default|GetPendingPlaneList)
      (if (== _array_element 0)
        (return _array_index 0)))
    (bind _returnvalue (Utilities|Array|Add _pendingplanelist _array_element))
    (return _returnvalue)
    (else
      (for (_array_element_2 _array_index_2) _pendingplanelist
        (if (not (== _array_element_2 0))
          (return _array_index_2 0)))
      (return -1 0))))