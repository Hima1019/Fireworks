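; FwoHoleMgr is a manager that drives the visibility and seed color of the hole components attached beneath it.
; BeginPlay caches the number of direct children as HuleMun.
; Every Tick maps EnableList by index onto each child's visibility, propagated to descendants.
; It then maps ColorList the same way, writing SeedColor on FwoSeed components found among each child's descendants.
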(event EventBeginPlay
  (Variables|Default|SetHuleMun (Utilities|Array|Length (Components|GetChildrenComponents false))))

(event EventTick
  (params (DeltaSeconds :type Float%20%28single-precision%29))
  ;[1 1 1] 描画切り替え
  (for (_array_element _array_index) (Variables|ボール設定|GetEnableList)
    (if (< _array_index (Variables|Default|GetHuleMun))
      (Rendering|SetVisibility (Utilities|Array|Get(acopy) (Components|GetChildrenComponents false) _array_index) _array_element true)))
  ;[1 1 1] カラー変更
  (for (_array_element_2 _array_index_2) (Variables|ボール設定|GetColorList)
    (if (< _array_index_2 (Variables|Default|GetHuleMun))
      ;;[1 1 1] Ball内
      (for _array_element_3 (Components|GetChildrenComponents (Utilities|Array|Get(acopy) (Components|GetChildrenComponents false) _array_index_2) true)
        (bind _asfwo_seed (Utilities|Casting|CastToFwoSeed _array_element_3))
        (Variables|/Game/BluePrints/OikawaBP/FwoSeed.FwoSeed_C|SetSeedColor _asfwo_seed _array_element_2)))))