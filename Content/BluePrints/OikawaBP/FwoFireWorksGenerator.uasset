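; Fireworks generator that turns a FwoPlane or a ball board into a firework and fires it from a launcher chosen by ID.
; BeginPlay caches all FwoFWLaunchers.
; Generator hides the plane's parts except Appearance, disables seed collision, adds the FireType's action component, moves it to the launcher and calls RequestFire.
; GeneratorToBaseBoard collects board balls, spawns a FwoPlane with their indices enabled, then repeats that setup and launch.
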(event EventBeginPlay
  (bind _outactors (Actor|GetAllActorsOfClass "/Game/BluePrints/OikawaBP/FwoFWLauncher.FwoFWLauncher_C"))
  (Variables|Default|SetLauncherArray _outactors))

(event EventActorBeginOverlap
  (params (OtherActor :type Actor%20Object%20Reference)))

(event EventTick
  (params (DeltaSeconds :type Float%20%28single-precision%29)))

(fn ConstructionScript)

(fn Generator
  (params (_Plane :type Fwo%20Plane%20Object%20Reference) (_LauncherId :type Integer))
  (bind _defaultsceneroot (Variables|/Game/BluePrints/OikawaBP/FwoPlane.FwoPlane_C|GetDefaultSceneRoot _Plane))
  (bind _children (Components|GetChildrenComponents _defaultsceneroot false))
  (LocalVariables|SetLauncherID _LauncherId)
  ;[1 1 1] 外見変更
  (for _array_element _children
    (Rendering|SetVisibility _array_element false true))
  (Rendering|SetVisibility (Variables|/Game/BluePrints/OikawaBP/FwoPlane.FwoPlane_C|GetAppearance _Plane) true false)
  (for _array_element_2 _children
    (bind _aschild_actor_component (Utilities|Casting|CastToChildActorComponent _array_element_2))
    (bind _asfwo_fire_seed (Utilities|Casting|CastToFwoFireSeed (Variables|/Script/Engine.ChildActorComponent|GetChildActor _aschild_actor_component)))
    (Collision|SetActorEnableCollision _asfwo_fire_seed false))
  ;[1 1 1] アクション設定
  (switch Utilities|FlowControl|Switch|SwitchonFwoFWActionEnum (Variables|/Game/BluePrints/OikawaBP/FwoPlane.FwoPlane_C|GetFireType _Plane)
    (:NewEnumerator0
      (bind _returnvalue (AddComponent|AddFwoAKIKUSAKI _Plane false))
      (Components|Activation|SetActive _returnvalue true false))
    (:NewEnumerator1
      (bind _returnvalue_2 (AddComponent|AddFwoABOTAN _Plane true))
      (Components|Activation|SetActive _returnvalue_2 true false))
    (:NewEnumerator2
      (bind _returnvalue_3 (AddComponent|AddFwoANISHIKIKAMURO _Plane false))
      (Components|Activation|SetActive _returnvalue_3 true false))
    (:NewEnumerator3
      (bind _returnvalue_4 (AddComponent|AddFwoAGINKAMURO _Plane false))
      (Components|Activation|SetActive _returnvalue_4 true false))
    (:NewEnumerator4
      (bind _returnvalue_5 (AddComponent|AddFwoAHIRAWARI _Plane false))
      (Components|Activation|SetActive _returnvalue_5 true false))
    (:NewEnumerator5
      (bind _returnvalue_6 (AddComponent|AddFwoASHINWARI _Plane false))
      (Components|Activation|SetActive _returnvalue_6 true false))
    (:NewEnumerator6
      (bind _returnvalue_7 (AddComponent|AddFwoAYAWSIN _Plane false))
      (Components|Activation|SetActive _returnvalue_7 true false)))
  ;[1 1 1] 発射地点移動
  (Transformation|SetActorRelativeLocation _Plane (Transformation|GetActorLocation (Utilities|Array|Get(acopy) (Variables|Default|GetLauncherArray) (LocalVariables|GetLauncherID))) false true)
  ;[1 1 1] 発射
  (Default|RequestFire (Utilities|Array|Get(acopy) (Variables|Default|GetLauncherArray) (LocalVariables|GetLauncherID)) _Plane))

(fn GeneratortoBaseBoard
  (params (_Base :type Fw%20Base%20Board%20Object%20Reference) (_LauncherId :type Integer))
  (Utilities|FlowControl|Sequence
    (:then_0
      (LocalVariables|SetLauncherID _LauncherId))
    (:then_1
      (for _array_element (Components|GetChildrenComponents (Variables|/Game/BluePrints/FwBaseBoard.FwBaseBoard_C|GetDefaultSceneRoot _Base) false)
        ;[1 1 1] 外郭非表示
        (bind _asスタティックメッシュコンポーネント (Utilities|Casting|CastToStaticMeshComponent _array_element)
          (:then
            (Rendering|SetVisibility _asスタティックメッシュコンポーネント false false))
          (:CastFailed
            ;[1 1 1] 有効なBall抽出
            (Utilities|Array|Clear (LocalVariables|GetinstantBallArray))
            (for _array_element_2 (Components|GetChildrenComponents (.AsFw%20Board%20Hole%20Mgr (Utilities|Casting|CastToFwBoardHoleMgr _array_element)) false)
              (if (Utilities|IsValid (Variables|/Script/Engine.ChildActorComponent|GetChildActor (.AsChild%20Actor%20Component (Utilities|Casting|CastToChildActorComponent _array_element_2))))
                (bind _returnvalue (Utilities|Array|Add (LocalVariables|GetinstantBallArray) (.AsFw%20Board%20Ball (Utilities|Casting|CastToFwBoardBall (Variables|/Script/Engine.ChildActorComponent|GetChildActor (.AsChild%20Actor%20Component (Utilities|Casting|CastToChildActorComponent _array_element_2)))))))))))))
    (:then_2
      (Actor|GetAllActorsOfClass "/Script/Engine.TargetPoint")
      (bind _returnvalue_2 (Game|SpawnActorfromClass "/Game/BluePrints/OikawaBP/FwoPlane.FwoPlane_C" (Math|Transform|MakeTransform (.Location (Math|Transform|BreakTransform (Transformation|GetActorTransform (Utilities|Array|Get(acopy) (Variables|Default|GetLauncherArray) (LocalVariables|GetLauncherID))))) "90.000000, 0, 0" (.Scale (Math|Transform|BreakTransform (Transformation|GetActorTransform (Utilities|Array|Get(acopy) (Variables|Default|GetLauncherArray) (LocalVariables|GetLauncherID)))))) "Undefined" 0 0))
      (Utilities|FlowControl|Sequence
        (:then_0
          ;[1 1 1] 色同期
          (for _array_element_3 (LocalVariables|GetinstantBallArray)
            (Utilities|Array|SetArrayElem (Variables|/Game/BluePrints/OikawaBP/FwoPlane.FwoPlane_C|GetColorArray _returnvalue_2) (Variables|/Game/BluePrints/FwBoardBall.FwBoardBall_C|GetIndexID _array_element_3) (Variables|/Game/BluePrints/OikawaBP/FwoFireSeed.FwoFireSeed_C|GetSeedColor (Utilities|Array|Get(acopy) (Variables|/Game/BluePrints/OikawaBP/FwoPlane.FwoPlane_C|GetFireSeedArray _returnvalue_2) (Variables|/Game/BluePrints/FwBoardBall.FwBoardBall_C|GetIndexID _array_element_3))))))
        (:then_1
          ;[1 1 1] 全隠蔽
          (for _array_element_4 (Variables|/Game/BluePrints/OikawaBP/FwoPlane.FwoPlane_C|GetFireSeedArray _returnvalue_2)
            (Rendering|SetVisibility (Variables|/Script/Engine.StaticMeshActor|GetStaticMeshComponent _array_element_4) false false)))
        (:then_2
          ;[1 1 1] 有効化リスト登録
          (for _array_element_5 (LocalVariables|GetinstantBallArray)
            (Utilities|Array|Add (Variables|/Game/BluePrints/OikawaBP/FwoPlane.FwoPlane_C|GetEnableArray _returnvalue_2) (Variables|/Game/BluePrints/FwBoardBall.FwBoardBall_C|GetIndexID _array_element_5))))
        (:then_3
          (Rendering|SetVisibility (Variables|/Game/BluePrints/OikawaBP/FwoPlane.FwoPlane_C|GetAppearance _returnvalue_2) true false)
          (for _array_element_6 (Components|GetChildrenComponents (Variables|/Game/BluePrints/OikawaBP/FwoPlane.FwoPlane_C|GetDefaultSceneRoot _returnvalue_2) false)
            (bind _aschild_actor_component (Utilities|Casting|CastToChildActorComponent _array_element_6))
            (bind _asfwo_fire_seed (Utilities|Casting|CastToFwoFireSeed (Variables|/Script/Engine.ChildActorComponent|GetChildActor _aschild_actor_component)))
            (Collision|SetActorEnableCollision _asfwo_fire_seed false))
          ;[1 1 1] アクション設定
          (switch Utilities|FlowControl|Switch|SwitchonFwoFWActionEnum (Variables|/Game/BluePrints/OikawaBP/FwoPlane.FwoPlane_C|GetFireType _returnvalue_2)
            (:NewEnumerator0
              (bind _returnvalue_3 (AddComponent|AddFwoAKIKUSAKI _returnvalue_2 false))
              (Components|Activation|SetActive _returnvalue_3 true false))
            (:NewEnumerator1
              (bind _returnvalue_4 (AddComponent|AddFwoABOTAN _returnvalue_2 true))
              (Components|Activation|SetActive _returnvalue_4 true false))
            (:NewEnumerator2
              (bind _returnvalue_5 (AddComponent|AddFwoANISHIKIKAMURO _returnvalue_2 false))
              (Components|Activation|SetActive _returnvalue_5 true false))
            (:NewEnumerator3
              (bind _returnvalue_6 (AddComponent|AddFwoAGINKAMURO _returnvalue_2 false))
              (Components|Activation|SetActive _returnvalue_6 true false))
            (:NewEnumerator4
              (bind _returnvalue_7 (AddComponent|AddFwoAHIRAWARI _returnvalue_2 false))
              (Components|Activation|SetActive _returnvalue_7 true false))
            (:NewEnumerator5
              (bind _returnvalue_8 (AddComponent|AddFwoASHINWARI _returnvalue_2 false))
              (Components|Activation|SetActive _returnvalue_8 true false))
            (:NewEnumerator6
              (bind _returnvalue_9 (AddComponent|AddFwoAYAWSIN _returnvalue_2 false))
              (Components|Activation|SetActive _returnvalue_9 true false)))
          ;[1 1 1] 発射地点移動
          (Transformation|SetActorRelativeLocation _returnvalue_2 (Transformation|GetActorLocation (Utilities|Array|Get(acopy) (Variables|Default|GetLauncherArray) (LocalVariables|GetLauncherID))) false true)
          ;[1 1 1] 発射
          (Default|RequestFire (Utilities|Array|Get(acopy) (Variables|Default|GetLauncherArray) (LocalVariables|GetLauncherID)) _returnvalue_2))))))