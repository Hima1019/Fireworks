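; Firework inner-burst actor that holds FwoFireSeed child actors and scatters them outward when fired.
; BeginPlay caches the seeds, a default color per seed and a center seed; insideFire moves to a given transform and impulses each seed away from center with an upward boost.
; Tick copies color and scale to seeds only while IsDeath is set.
; Death destroys the seeds and itself; helpers reset colors and decrement Life.
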(event Custom|Death
  ;[1 1 1] 削除
  (for _array_element (Components|GetChildrenComponents (Variables|Components|GetDefaultSceneRoot) false)
    (bind _aschild_actor_component (Utilities|Casting|CastToChildActorComponent _array_element))
    (bind _asfwo_fire_seed (Utilities|Casting|CastToFwoFireSeed (Variables|/Script/Engine.ChildActorComponent|GetChildActor _aschild_actor_component)))
    (Actor|DestroyActor _asfwo_fire_seed))
  (Actor|DestroyActor)
  (Variables|Default|SetisDeath true))

(event Custom|insideFire
  (params (trans :type Transform))
  (bind (_location _rotation) (Math|Transform|BreakTransform trans))
  ;[1 1 1] 発射
  (Transformation|SetActorLocation _location false false)
  (Transformation|SetActorRotation _rotation)
  (for _array_element (Variables|Default|GetFireSeedArray)
    (bind _output_get (Variables|Default|Setimpulse (- (Transformation|GetWorldLocation (Variables|/Script/Engine.StaticMeshActor|GetStaticMeshComponent _array_element)) (Transformation|GetWorldLocation (Variables|/Script/Engine.StaticMeshActor|GetStaticMeshComponent (Variables|Default|GetCenter))))))
    ;;[1 1 1] 加力
    (Physics|AddImpulse (Variables|/Script/Engine.StaticMeshActor|GetStaticMeshComponent _array_element) (+ (* _output_get (Variables|Default|GetmulForce)) "0,0.000000,100.000000") "None" false)))

(event EventBeginPlay
  ;[1 1 1] アクター所得
  (for _array_element (Components|GetChildrenComponents (Variables|Components|GetDefaultSceneRoot) false)
    (bind _aschild_actor_component (Utilities|Casting|CastToChildActorComponent _array_element))
    (bind _asfwo_fire_seed (Utilities|Casting|CastToFwoFireSeed (Variables|/Script/Engine.ChildActorComponent|GetChildActor _aschild_actor_component)))
    (Utilities|Array|Add (Variables|Default|GetFireSeedArray) _asfwo_fire_seed)
    ;[1 1 1] 色初期化
    (Utilities|Array|Add (Variables|Default|GetColorArray) (Variables|Default|GetDefaultColor)))
  ;[1 1 1] 中心設定
  (bind _asfwo_fire_seed_2 (Utilities|Casting|CastToFwoFireSeed (Variables|/Script/Engine.ChildActorComponent|GetChildActor (Variables|Seeds|GetChildSeed))))
  (Variables|Default|SetCenter _asfwo_fire_seed_2))

(event EventTick
  (params (DeltaSeconds :type Float%20%28single-precision%29))
  (if (Variables|Default|GetisDeath)
    ;[1 1 1] カラー更新
    (for (_array_element _array_index) (Variables|Default|GetColorArray)
      (if (Utilities|IsValid (Utilities|Array|Get(acopy) (Variables|Default|GetFireSeedArray) _array_index))
        (Variables|/Game/BluePrints/OikawaBP/FwoFireSeed.FwoFireSeed_C|SetSeedColor (Utilities|Array|Get(acopy) (Variables|Default|GetFireSeedArray) _array_index) _array_element)
        (Variables|/Game/BluePrints/OikawaBP/FwoFireSeed.FwoFireSeed_C|SetSeedScale (Utilities|Array|Get(acopy) (Variables|Default|GetFireSeedArray) _array_index) (Variables|Default|GetSeedScale))))))

(fn ConstructionScript)

(fn ResetColor
  (bind _colorarray (Variables|Default|GetColorArray))
  ;[1 1 1] カラー初期化
  (for (_ _array_index) _colorarray
    (Utilities|Array|SetArrayElem _colorarray _array_index (Variables|Default|GetDefaultColor))))

(fn LifeDamege
  (Math|Integer|DecrementInt (Variables|Default|GetLife)))