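; FwoStock is an actor that displays a firework stock ball on a Sphere mesh, styled by firework type and color.
; Its Make function creates a dynamic material from M_TexBall_Inst and sets BaseColor from the passed color.
; A switch on the firework type enum then assigns the matching Kayaku texture.
; Event graph and construction script are empty, so the look changes only when Make is called.
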(event EventBeginPlay)

(event EventActorBeginOverlap
  (params (OtherActor :type Actor%20Object%20Reference)))

(event EventTick
  (params (DeltaSeconds :type Float%20%28single-precision%29)))

(fn ConstructionScript)

(fn Make
  (params (NewParam :type FwoFWActionEnum%20Enum) (NewParam1 :type Linear%20Color%20Structure))
  (bind _returnvalue (Rendering|Material|CreateDynamicMaterialInstance (Variables|Default|GetSphere) 0 "/Game/Architecture/Materials/M_TexBall_Inst.M_TexBall_Inst" :!class /Script/Engine.PrimitiveComponent))
  (bind _output_get (Variables|Default|SetDynamicMaterial _returnvalue))
  (Rendering|Material|SetVectorParameterValue _output_get "BaseColor" NewParam1 :!class /Script/Engine.MaterialInstanceDynamic)
  (switch Utilities|FlowControl|Switch|SwitchonFwoFWActionEnum NewParam
    (:NewEnumerator0
      (Rendering|Material|SetTextureParameterValue (Variables|Default|GetDynamicMaterial) "Texture" "/Game/Architecture/Textures/kayaku01.kayaku01"))
    (:NewEnumerator1
      (Rendering|Material|SetTextureParameterValue (Variables|Default|GetDynamicMaterial) "Texture" "/Game/Architecture/Textures/kayaku02.kayaku02"))
    (:NewEnumerator2
      (Rendering|Material|SetTextureParameterValue (Variables|Default|GetDynamicMaterial) "Texture" "/Game/Architecture/Textures/kayaku03.kayaku03"))
    (:NewEnumerator3
      (Rendering|Material|SetTextureParameterValue (Variables|Default|GetDynamicMaterial) "Texture" "/Game/Architecture/Textures/kayaku05.kayaku05"))
    (:NewEnumerator4
      (Rendering|Material|SetTextureParameterValue (Variables|Default|GetDynamicMaterial) "Texture" "/Game/Architecture/Textures/kayaku04.kayaku04"))
    (:NewEnumerator5
      (Rendering|Material|SetTextureParameterValue (Variables|Default|GetDynamicMaterial) "Texture" "/Game/Architecture/Textures/kayaku06.kayaku06"))))