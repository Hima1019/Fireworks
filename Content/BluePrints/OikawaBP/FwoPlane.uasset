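; FwoPlane is a firework actor that groups FwoFireSeed child actors around a center seed and manages their color, scale and cleanup.
; BeginPlay gathers the seeds, sets Life to their count and hides the Appearance component.
; Tick moves Appearance to the center seed, pushes per-seed color and shared scale, and creates a dynamic material instance to set Emit.
; Death destroys seeds and actor; helpers reset colors and decrement Life.
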(event Custom|Death
  (for _array_element (Components|GetChildrenComponents (Variables|Components|GetDefaultSceneRoot) false)
    (bind _aschild_actor_component (Utilities|Casting|CastToChildActorComponent _array_element))
    (bind _asfwo_fire_seed (Utilities|Casting|CastToFwoFireSeed (Variables|/Script/Engine.ChildActorComponent|GetChildActor _aschild_actor_component)))
    (Actor|DestroyActor _asfwo_fire_seed))
  (Actor|DestroyActor)
  (Variables|Default|SetisDeath true))

(event EventBeginPlay
  ;[1 1 1] アクター所得
  (for _array_element (Components|GetChildrenComponents (Variables|Components|GetDefaultSceneRoot) false)
    (bind _aschild_actor_component (Utilities|Casting|CastToChildActorComponent _array_element))
    (bind _asfwo_fire_seed (Utilities|Casting|CastToFwoFireSeed (Variables|/Script/Engine.ChildActorComponent|GetChildActor _aschild_actor_component)))
    (Utilities|Array|Add (Variables|Default|GetFireSeedArray) _asfwo_fire_seed)
    ;[1 1 1] 色初期化
    (Utilities|Array|Add (Variables|Default|GetColorArray) (Variables|Default|GetDefaultColor)))
  ;[1 1 1] 中心設定
  (bind _asfwo_fire_seed_2 (Utilities|Casting|CastToFwoFireSeed (Variables|/Script/Engine.ChildActorComponent|GetChildActor (Variables|Seeds|GetChildSeed))))
  (Variables|Default|SetCenter _asfwo_fire_seed_2)
  ;[1 1 1] 外見参照取得
  (Rendering|SetVisibility (Variables|Components|GetAppearance) false false)
  (Variables|Default|SetLife (Utilities|Array|Length (Variables|Default|GetFireSeedArray))))

(event EventTick
  (params (DeltaSeconds :type Float%20%28single-precision%29))
  (if (not (Variables|Default|GetisDeath))
    ;[1 1 1] 同期
    (Transformation|SetRelativeLocation (Variables|Components|GetAppearance) (Transformation|GetActorLocation (Variables|Default|GetCenter)) false false)
    ;[1 1 1] カラー更新
    (for (_array_element _array_index) (Variables|Default|GetColorArray)
      (if (Utilities|IsValid (Utilities|Array|Get(acopy) (Variables|Default|GetFireSeedArray) _array_index))
        (Variables|/Game/BluePrints/OikawaBP/FwoFireSeed.FwoFireSeed_C|SetSeedColor (Utilities|Array|Get(acopy) (Variables|Default|GetFireSeedArray) _array_index) _array_element)
        (Variables|/Game/BluePrints/OikawaBP/FwoFireSeed.FwoFireSeed_C|SetSeedScale (Utilities|Array|Get(acopy) (Variables|Default|GetFireSeedArray) _array_index) (Variables|Default|GetSeedScale))))
    ;[1 1 1] 光量変更
    (bind _returnvalue (Rendering|Material|CreateDynamicMaterialInstance (Variables|Components|GetAppearance) 0 "/Game/Architecture/Materials/Mo_hanabidama_Inst.Mo_hanabidama_Inst" :!class /Script/Engine.PrimitiveComponent))
    (Rendering|Material|SetScalarParameterValue _returnvalue "Emit" (Variables|Default|GetAppearanceEmit) :!class /Script/Engine.MaterialInstanceDynamic)))

(fn ConstructionScript)

(fn ResetColor
  (bind _colorarray (Variables|Default|GetColorArray))
  ;[1 1 1] カラー初期化
  (for (_ _array_index) _colorarray
    (Utilities|Array|SetArrayElem _colorarray _array_index (Variables|Default|GetDefaultColor))))

(fn LifeDamege
  (Math|Integer|DecrementInt (Variables|Default|GetLife)))