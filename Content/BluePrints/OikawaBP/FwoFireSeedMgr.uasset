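; Manager for firework seeds that controls the visibility and color of its child balls and the FwoSeed components under them.
; On BeginPlay it counts its child balls and gathers their direct FwoSeed children into Seeds.
; Every Tick it applies EnableList to each ball's visibility, propagated to its children, and writes ColorList into SeedColor on that ball's descendant seeds.
; Both lists map by child index, and Tick re-queries the hierarchy rather than using the cached Seeds.
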(event EventBeginPlay
  (bind _children (Components|GetChildrenComponents false))
  ;[1 1 1] ボール数取得
  (Variables|ボール設定|SetBallNum (Utilities|Array|Length _children))
  ;[1 1 1] Mgr>Ball>Seedを取得
  (for _array_element _children
    (for _array_element_2 (Components|GetChildrenComponents _array_element false)
      (bind _asfwo_seed (Utilities|Casting|CastToFwoSeed _array_element_2))
      (Utilities|Array|Add (Variables|Default|GetSeeds) _asfwo_seed))))

(event EventTick
  (params (DeltaSeconds :type Float%20%28single-precision%29))
  ;[1 1 1] 描画切り替え
  (for (_array_element _array_index) (Variables|ボール設定|GetEnableList)
    (if (< _array_index (Variables|ボール設定|GetBallNum))
      (Rendering|SetVisibility (Utilities|Array|Get(acopy) (Components|GetChildrenComponents false) _array_index) _array_element true)))
  ;[1 1 1] カラー変更
  (for (_array_element_2 _array_index_2) (Variables|ボール設定|GetColorList)
    (if (< _array_index_2 (Variables|ボール設定|GetBallNum))
      ;;[1 1 1] Ball内
      (for _array_element_3 (Components|GetChildrenComponents (Utilities|Array|Get(acopy) (Components|GetChildrenComponents false) _array_index_2) true)
        (bind _asfwo_seed (Utilities|Casting|CastToFwoSeed _array_element_3))
        (Variables|/Game/BluePrints/OikawaBP/FwoSeed.FwoSeed_C|SetSeedColor _asfwo_seed _array_element_2)))))